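; ExplosiveBarrelBP is an explosive barrel actor that detonates on a server-started timer a few seconds after BeginPlay.
; Only the authority starts the timer, whose Explode event calls MultiCastExplode and sets a short lifespan to remove the actor.
; MultiCastExplode prints a debug string, fires the RadialForce impulse and disables collision, while its SetActorHiddenInGame call passes false, leaving the barrel visible.
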(event Custom|MultiCastExplode
  (Development|PrintString "EXPLODE")
  (Class|RadialForceComponent|FireImpulse (Variables|Default|GetRadialForce))
  (Rendering|SetActorHiddenInGame false)
  (Collision|SetActorEnableCollision false))

(event Custom|Explode
  (CallFunction|MultiCastExplode)
  (Actor|SetLifeSpan 2.0))

(event EventBeginPlay
  (if (Ability|HasAuthority)
    (Utilities|Time|SetTimerbyEvent (delegate Custom|Explode) 4.0)))

(fn ConstructionScript)